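; BP_Enemy_Zombie is a zombie enemy that dies from a single projectile hit.
; Each Tick it moves 2 units down world Z with sweep, a frame-rate-dependent speed, and polls for overlapping BP_ProjectileBase actors rather than using overlap events.
; On a hit it spawns BP_Combat_HitExplosion at the first projectile's location, then destroys that projectile and itself.
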(event EventTick
  (params (DeltaSeconds :type Float%20%28single-precision%29))
  (bind _overlappingactors (Collision|GetOverlappingActors "/Game/Blueprints/Combat/Projectiles/BP_ProjectileBase.BP_ProjectileBase_C" :!class /Script/Engine.Actor))
  (bind _item (Utilities|Array|Get(acopy) _overlappingactors))
  (bind _returnvalue (Transformation|GetActorLocation _item))
  (bind _returnvalue_2 (Math|Transform|MakeTransform _returnvalue))
  (Transformation|AddActorWorldOffset "0,0,-2.0" true)
  (if (> (Utilities|Array|Length _overlappingactors) 0)
    (bind _returnvalue_3 (Class|GameplayStatics|BeginDeferredActorSpawnfromClass "/Game/Blueprints/Combat/Projectiles/BP_Combat_HitExplosion.BP_Combat_HitExplosion_C" _returnvalue_2 "Undefined" 0 "MultiplyWithRoot"))
    (Class|GameplayStatics|FinishSpawningActor _returnvalue_3 _returnvalue_2 "MultiplyWithRoot")
    (Actor|DestroyActor _item)
    (Actor|DestroyActor)))

(fn ConstructionScript)