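; Base combat projectile actor that damages what it overlaps and destroys itself after a short lifetime.
; On overlap it ignores actors tagged Player and the pawn controlled by the first player controller.
; For any other actor it spawns a hit explosion at its location and a damage pop slightly above, applies fixed damage, then destroys itself.
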(event EventBeginPlay
  (Utilities|FlowControl|Delay 2.0)
  (Actor|DestroyActor))

(event Collision|EventActorBeginOverlap
  (params (OtherActor :type Actor%20Object%20Reference))
  (bind _returnvalue (Transformation|GetActorLocation))
  (bind _returnvalue_2 (Math|Transform|MakeTransform _returnvalue))
  (bind (_x _y _z) (Math|Vector|BreakVector _returnvalue))
  (bind _returnvalue_3 (+ _z 35.0))
  (bind _returnvalue_4 (Math|Vector|MakeVector _x _y _returnvalue_3))
  (bind _returnvalue_5 (Math|Transform|MakeTransform _returnvalue_4))
  (if (not (or (Actor|ActorHasTag OtherActor "Player") (== OtherActor (Pawn|GetControlledPawn (Game|GetPlayerController 0)))))
    (bind _returnvalue_6 (Class|GameplayStatics|BeginDeferredActorSpawnfromClass "/Game/Blueprints/Combat/Projectiles/BP_Combat_HitExplosion.BP_Combat_HitExplosion_C" _returnvalue_2 "Undefined" 0 "MultiplyWithRoot"))
    (Class|GameplayStatics|FinishSpawningActor _returnvalue_6 _returnvalue_2 "MultiplyWithRoot")
    (bind _returnvalue_7 (Class|GameplayStatics|BeginDeferredActorSpawnfromClass "/Game/Blueprints/Combat/Projectiles/BP_Combat_DamagePop.BP_Combat_DamagePop_C" _returnvalue_5 "Undefined" 0 "MultiplyWithRoot"))
    (Class|GameplayStatics|FinishSpawningActor _returnvalue_7 _returnvalue_5 "MultiplyWithRoot")
    (Game|Damage|ApplyDamage OtherActor 45.0 0 0)
    (Actor|DestroyActor)))

(fn ConstructionScript)