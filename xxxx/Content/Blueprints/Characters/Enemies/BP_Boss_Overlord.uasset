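; Paper2D Overlord boss enemy that pursues the player on the X/Z plane and loses health when damaged.
; Tick moves it with swept offsets, choosing a walk flipbook by dominant axis, or the downward slam flipbook at close range.
; AnyDamage reduces health and rescales the world-space bar actor tagged BossBarFill, or on death destroys the boss and four BossBarGroup actors.
; The overlap event has no effect.
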(event EventBeginPlay)

(event Game|Damage|EventAnyDamage
  (params (Damage :type Float%20%28single-precision%29) (DamageType :type Damage%20Type%20Object%20Reference) (InstigatedBy :type Controller%20Object%20Reference) (DamageCauser :type Actor%20Object%20Reference))
  (Variables|战斗属性|SetCurrentHealth (Math|Float|Max(Float) (- (Variables|战斗属性|GetCurrentHealth) Damage) 0.0))
  (if (<= (Math|Float|Max(Float) (- (Variables|战斗属性|GetCurrentHealth) Damage) 0.0) 0.0)
    (Collision|SetActorEnableCollision false)
    (Rendering|SetActorHiddenInGame true)
    (bind _outactors (Actor|GetAllActorswithTag "BossBarGroup"))
    (Rendering|SetActorHiddenInGame (Utilities|Array|Get(acopy) _outactors) true)
    (Actor|DestroyActor (Utilities|Array|Get(acopy) _outactors))
    (Rendering|SetActorHiddenInGame (Utilities|Array|Get(acopy) _outactors 1) true)
    (Actor|DestroyActor (Utilities|Array|Get(acopy) _outactors 1))
    (Rendering|SetActorHiddenInGame (Utilities|Array|Get(acopy) _outactors 2) true)
    (Actor|DestroyActor (Utilities|Array|Get(acopy) _outactors 2))
    (Rendering|SetActorHiddenInGame (Utilities|Array|Get(acopy) _outactors 3) true)
    (Actor|DestroyActor (Utilities|Array|Get(acopy) _outactors 3))
    (Actor|DestroyActor)
    (else
      (bind _outactors_2 (Actor|GetAllActorswithTag "BossBarFill"))
      (Transformation|SetActorScale3D (Utilities|Array|Get(acopy) _outactors_2) (Math|Vector|MakeVector (* (Math|Float|Clamp(Float) (/ (Math|Float|Max(Float) (- (Variables|战斗属性|GetCurrentHealth) Damage) 0.0) 1.2e+03)) 0.2) 1.0 0.16)))))

(event EventTick
  (params (DeltaSeconds :type Float%20%28single-precision%29))
  (bind _returnvalue (Game|Player|GetPlayerPawn 0))
  (bind _returnvalue_2 (Transformation|GetActorLocation))
  (bind _returnvalue_3 (Actor|GetComponentbyClass "/Script/Paper2D.PaperFlipbookComponent"))
  (bind _returnvalue_4 (Transformation|GetActorLocation _returnvalue))
  (bind _returnvalue_5 (- _returnvalue_4 _returnvalue_2))
  (bind _returnvalue_6 (Math|Vector|Normalize _returnvalue_5))
  (bind (_x _y _z) (Math|Vector|BreakVector _returnvalue_6))
  (if (> (Math|Vector|Distance(Vector) _returnvalue_4 _returnvalue_2) 1.5e+02)
    (Transformation|AddActorWorldOffset (Math|Vector|MakeVector (* (* _x 5e+01) DeltaSeconds) 0.0 0.0) true)
    (Transformation|AddActorWorldOffset (Math|Vector|MakeVector 0.0 0.0 (* (* _z 5e+01) DeltaSeconds)) true)
    (if (> (Math|Float|Absolute(Float) _x) (Math|Float|Absolute(Float) _z))
      (if (> _x 0.0)
        (Sprite|SetFlipbook _returnvalue_3 "/Game/P01/Imported/Content/Asset/Art/02_Enemies/Boss_Overlord/Actions/Walk/Dir_02_Right/Flipbooks/FB_T_Boss_Walk_Dir_02_Right_Sheet.FB_T_Boss_Walk_Dir_02_Right_Sheet")
        (else
          (Sprite|SetFlipbook _returnvalue_3 "/Game/P01/Imported/Content/Asset/Art/02_Enemies/Boss_Overlord/Actions/Walk/Dir_04_Left/Flipbooks/FB_T_Boss_Walk_Dir_04_Left_Sheet.FB_T_Boss_Walk_Dir_04_Left_Sheet")))
      (elif (> _z 0.0)
        (Sprite|SetFlipbook _returnvalue_3 "/Game/P01/Imported/Content/Asset/Art/02_Enemies/Boss_Overlord/Actions/Walk/Dir_03_Up/Flipbooks/FB_T_Boss_Walk_Dir_03_Up_Sheet.FB_T_Boss_Walk_Dir_03_Up_Sheet")
        (else
          (Sprite|SetFlipbook _returnvalue_3 "/Game/P01/Imported/Content/Asset/Art/02_Enemies/Boss_Overlord/Actions/Walk/Dir_01_Down/Flipbooks/FB_T_Boss_Walk_Dir_01_Down_Sheet.FB_T_Boss_Walk_Dir_01_Down_Sheet"))))
    (else
      (Sprite|SetFlipbook _returnvalue_3 "/Game/P01/Imported/Content/Asset/Art/02_Enemies/Boss_Overlord/Actions/Ground_Slam/Dir_01_Down/Flipbooks/FB_T_Boss_Slam_Dir_01_Down_Sheet.FB_T_Boss_Slam_Dir_01_Down_Sheet"))))

(event Collision|EventActorBeginOverlap
  (params (OtherActor :type Actor%20Object%20Reference))
  (if (!= OtherActor (Game|Player|GetPlayerPawn 0))
    _))

(fn ConstructionScript)