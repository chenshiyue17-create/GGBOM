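; BP_ENE_ZombieWalker is a zombie enemy whose Paper2D flipbook turns to face the player.
; Each Tick mirrors the flipbook's X scale according to which side the player pawn is on.
; An unswept world offset follows the normalized direction to the player, but its zero-vector multiplier leaves the walker in place.
; A duplicate of this logic is never run, and construction is empty.
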(event EventBeginPlay)

(event Collision|EventActorBeginOverlap
  (params (OtherActor :type Actor%20Object%20Reference)))

(event EventTick
  (params (DeltaSeconds :type Float%20%28single-precision%29))
  (bind _returnvalue (Game|Player|GetPlayerPawn 0))
  (bind _returnvalue_2 (Transformation|GetActorLocation))
  (bind _returnvalue_3 (Transformation|GetActorLocation _returnvalue))
  (bind _returnvalue_4 (- _returnvalue_3 _returnvalue_2))
  (if (Utilities|IsValid _returnvalue)
    (Transformation|AddActorWorldOffset (* (* (Math|Vector|Normalize _returnvalue_4) "") DeltaSeconds))
    (Transformation|SetRelativeScale3D (Actor|GetComponentbyClass "/Script/Paper2D.PaperFlipbookComponent") (Math|Vector|MakeVector (Math|Float|SelectFloat -0.45 0.45 (< (.X (Math|Vector|BreakVector _returnvalue_4)) 0.0)) 0.45 0.45))))

(fn ConstructionScript)