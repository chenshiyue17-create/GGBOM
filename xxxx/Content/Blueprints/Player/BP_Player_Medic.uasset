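; Medic player actor for a Paper2D game on the X/Z plane, with directional animation and automatic shooting.
; BeginPlay switches view to a level CameraActor; Tick polls WASD, updating facing, swept movement and idle/run flipbooks, mirroring side sprites by scale.
; A cooldown timer spawns BP_ProjectileBase along the facing direction without fire input.
; SampleMoveInput multiplies normalized input by a zero vector, so movement and facing never change as written.
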(event EventBeginPlay
  (bind _returnvalue (Actor|GetActorOfClass "/Script/Engine.CameraActor"))
  (Game|Player|SetViewTargetwithBlend (Game|GetPlayerController 0) _returnvalue 0.0 "VTBlend_Linear" 0.0 false))

(event EventTick
  (params (DeltaSeconds :type Float%20%28single-precision%29))
  (CallFunction|SampleMoveInput)
  (CallFunction|UpdateFacingDirection)
  (Transformation|AddActorWorldOffset (Variables|DirectionState|GetMoveInput) true)
  (CallFunction|UpdateFacingScale)
  (CallFunction|UpdateFireCooldown)
  (CallFunction|UpdateRunAnimation)
  (CallFunction|UpdateIdleAnimation)
  (CallFunction|TryFireProjectile))

(fn ConstructionScript)

(fn SampleMoveInput
  (bind _returnvalue (Game|GetPlayerController 0))
  (Variables|DirectionState|SetMoveInput (* (Math|Vector|Normalize (Math|Vector|MakeVector (+ (Math|Float|SelectFloat 7.5 0.0 (Game|Player|IsInputKeyDown _returnvalue "A")) (Math|Float|SelectFloat -7.5 0.0 (Game|Player|IsInputKeyDown _returnvalue "D"))) 0.0 (+ (Math|Float|SelectFloat 7.5 0.0 (Game|Player|IsInputKeyDown _returnvalue "W")) (Math|Float|SelectFloat -7.5 0.0 (Game|Player|IsInputKeyDown _returnvalue "S"))))) "")))

(fn UpdateFacingDirection
  (bind _moveinput (Variables|DirectionState|GetMoveInput))
  (Variables|DirectionState|SetFacingDirection (Math|Vector|SelectVector _moveinput (Variables|DirectionState|GetFacingDirection) (not (Math|Vector|VectorIsNearlyZero _moveinput 0.0001)))))

(fn UpdateFacingScale
  (Transformation|SetRelativeScale3D (Actor|GetComponentbyClass "/Script/Paper2D.PaperFlipbookComponent") (Math|Vector|MakeVector (Math|Float|SelectFloat -0.45 0.45 (< (.X (Math|Vector|BreakVector (Variables|DirectionState|GetFacingDirection))) 0.0)) 0.45 0.45)))

(fn UpdateRunAnimation
  (bind _returnvalue (Actor|GetComponentbyClass "/Script/Paper2D.PaperFlipbookComponent"))
  (bind _facingdirection (Variables|DirectionState|GetFacingDirection))
  (bind (_x _y _z) (Math|Vector|BreakVector _facingdirection))
  (if (not (Math|Vector|VectorIsNearlyZero (Variables|DirectionState|GetMoveInput) 0.0001))
    (if (> (Math|Float|Absolute(Float) _x) (Math|Float|Absolute(Float) _z))
      (Sprite|SetFlipbook _returnvalue "/Game/P01/Imported/Content/Asset/Art/01_Player/01_Idle_Run/Dir_03_Left/Run/Flipbooks/FB_T_Player_Medic_Run_Dir_03_Left_Sheet.FB_T_Player_Medic_Run_Dir_03_Left_Sheet")
      (elif (> _z 0.0)
        (Sprite|SetFlipbook _returnvalue "/Game/P01/Imported/Content/Asset/Art/01_Player/01_Idle_Run/Dir_05_Up/Run/Flipbooks/FB_T_Player_Medic_Run_Dir_05_Up_Sheet.FB_T_Player_Medic_Run_Dir_05_Up_Sheet")
        (else
          (Sprite|SetFlipbook _returnvalue "/Game/P01/Imported/Content/Asset/Art/01_Player/01_Idle_Run/Dir_01_Down/Run/Flipbooks/FB_T_Player_Medic_Run_Dir_01_Down_Sheet.FB_T_Player_Medic_Run_Dir_01_Down_Sheet"))))))

(fn UpdateIdleAnimation
  (bind _returnvalue (Actor|GetComponentbyClass "/Script/Paper2D.PaperFlipbookComponent"))
  (bind _facingdirection (Variables|DirectionState|GetFacingDirection))
  (bind (_x _y _z) (Math|Vector|BreakVector _facingdirection))
  (if (Math|Vector|VectorIsNearlyZero (Variables|DirectionState|GetMoveInput) 0.0001)
    (if (> (Math|Float|Absolute(Float) _x) (Math|Float|Absolute(Float) _z))
      (Sprite|SetFlipbook _returnvalue "/Game/P01/Imported/Content/Asset/Art/01_Player/01_Idle_Run/Dir_03_Left/Idle/Flipbooks/FB_T_Player_Medic_Idle_Dir_03_Left_Sheet.FB_T_Player_Medic_Idle_Dir_03_Left_Sheet")
      (elif (> _z 0.0)
        (Sprite|SetFlipbook _returnvalue "/Game/P01/Imported/Content/Asset/Art/01_Player/01_Idle_Run/Dir_05_Up/Idle/Flipbooks/FB_T_Player_Medic_Idle_Dir_05_Up_Sheet.FB_T_Player_Medic_Idle_Dir_05_Up_Sheet")
        (else
          (Sprite|SetFlipbook _returnvalue "/Game/P01/Imported/Content/Asset/Art/01_Player/01_Idle_Run/Dir_01_Down/Idle/Flipbooks/FB_T_Player_Medic_Idle_Dir_01_Down_Sheet.FB_T_Player_Medic_Idle_Dir_01_Down_Sheet"))))))

(fn UpdateFireCooldown
  (Variables|DirectionState|SetFireCooldownRemaining (Math|Float|SelectFloat (- (Variables|DirectionState|GetFireCooldownRemaining) (Utilities|Time|GetWorldDeltaSeconds)) 0.0 (> (- (Variables|DirectionState|GetFireCooldownRemaining) (Utilities|Time|GetWorldDeltaSeconds)) 0.0))))

(fn SpawnDirectionalProjectile
  (bind _returnvalue (Transformation|GetActorLocation))
  (bind _shotdirection (Variables|DirectionState|GetShotDirection))
  (bind _returnvalue_2 (Math|Rotator|MakeRotfromX _shotdirection))
  (bind _returnvalue_3 (+ _returnvalue _shotdirection))
  (bind _returnvalue_4 (+ _returnvalue_3 "0,-5,55"))
  (bind _returnvalue_5 (Math|Transform|MakeTransform _returnvalue_4 _returnvalue_2 "1,1,1"))
  (bind _returnvalue_6 (Class|GameplayStatics|BeginDeferredActorSpawnfromClass "/Game/Blueprints/Combat/Projectiles/BP_ProjectileBase.BP_ProjectileBase_C" _returnvalue_5 "Undefined" 0 "MultiplyWithRoot"))
  (Class|GameplayStatics|FinishSpawningActor _returnvalue_6 _returnvalue_5 "MultiplyWithRoot"))

(fn TryFireProjectile
  (if (<= (Variables|DirectionState|GetFireCooldownRemaining) 0.0)
    (Variables|DirectionState|SetFireCooldownRemaining (Variables|DirectionState|GetFireCooldown))
    (Variables|DirectionState|SetShotDirection (Variables|DirectionState|GetFacingDirection))
    (CallFunction|SpawnDirectionalProjectile)))