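; BP_ProjectileBase is a projectile actor, named as a base class, that destroys itself after a fixed delay from BeginPlay.
; Tick offsets it along its forward vector without sweep, but the velocity multiplier is a zero vector, so that offset produces no movement.
; Overlap handling is disabled and the construction script is empty.
; Disconnected leftover nodes hold alternative lifetime timers and a local-space forward movement step.
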(event EventBeginPlay
  (Utilities|FlowControl|Delay 3.5)
  (Actor|DestroyActor))

(event Collision|EventActorBeginOverlap
  (params (OtherActor :type Actor%20Object%20Reference)))

(event EventTick
  (params (DeltaSeconds :type Float%20%28single-precision%29))
  (Transformation|AddActorWorldOffset (* (* (Transformation|GetActorForwardVector) "") DeltaSeconds)))

(fn ConstructionScript)