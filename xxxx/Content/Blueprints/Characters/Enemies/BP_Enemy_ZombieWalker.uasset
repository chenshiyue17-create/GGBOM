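; Zombie walker enemy that chases player 0 in the X-Z plane using a Paper2D flipbook.
; Each Tick it takes swept steps toward a point horizontally offset on its side of the player until within stopping range, mirroring the flipbook by X direction.
; Overlapping actors other than the player push it away.
; Damage lowers CurrentHealth, but the death check subtracts Damage again, so it can be destroyed with health remaining.
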(event EventBeginPlay)

(event Collision|EventActorBeginOverlap
  (params (OtherActor :type Actor%20Object%20Reference))
  (if (!= OtherActor (Game|Player|GetPlayerPawn 0))
    (Transformation|AddActorWorldOffset (* (Math|Vector|Normalize (- (Transformation|GetActorLocation) (Transformation|GetActorLocation OtherActor))) "40.0, 0.0, 40.0"))))

(event EventTick
  (params (DeltaSeconds :type Float%20%28single-precision%29))
  (bind _returnvalue (Game|Player|GetPlayerPawn 0))
  (bind _returnvalue_2 (Transformation|GetActorLocation))
  (bind _returnvalue_3 (Actor|GetComponentbyClass "/Script/Paper2D.PaperFlipbookComponent"))
  (bind _returnvalue_4 (Transformation|GetActorLocation _returnvalue))
  (bind _returnvalue_5 (- _returnvalue_2 _returnvalue_4))
  (bind _x (Math|Vector|BreakVector _returnvalue_5))
  (bind _returnvalue_6 (Math|Vector|MakeVector _x 0.0 0.0))
  (bind _returnvalue_7 (Math|Vector|Normalize _returnvalue_6))
  (bind _returnvalue_8 (* _returnvalue_7 "45.0, 0.0, 30.0"))
  (bind _returnvalue_9 (+ _returnvalue_4 _returnvalue_8))
  (bind _returnvalue_10 (- _returnvalue_9 _returnvalue_2))
  (bind _returnvalue_11 (Math|Vector|Normalize _returnvalue_10))
  (bind (_x_2 _y _z) (Math|Vector|BreakVector _returnvalue_11))
  (if (> (Math|Vector|Distance(Vector) _returnvalue_9 _returnvalue_2) 95.0)
    (Transformation|AddActorWorldOffset (Math|Vector|MakeVector (* (* _x_2 65.0) DeltaSeconds) 0.0 0.0) true)
    (Transformation|AddActorWorldOffset (Math|Vector|MakeVector 0.0 0.0 (* (* _z 65.0) DeltaSeconds)) true)
    (if (> _x_2 0.0)
      (Transformation|SetRelativeScale3D _returnvalue_3 "-0.45, 0.45, 0.45")
      (else
        (Transformation|SetRelativeScale3D _returnvalue_3 "0.45, 0.45, 0.45")))))

(event Game|Damage|EventAnyDamage
  (params (Damage :type Float%20%28single-precision%29) (DamageType :type Damage%20Type%20Object%20Reference) (InstigatedBy :type Controller%20Object%20Reference) (DamageCauser :type Actor%20Object%20Reference))
  (Variables|战斗属性|SetCurrentHealth (- (Variables|战斗属性|GetCurrentHealth) Damage))
  (if (<= (- (Variables|战斗属性|GetCurrentHealth) Damage) 0.0)
    (Actor|DestroyActor)))

(fn ConstructionScript)