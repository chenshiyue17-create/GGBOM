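; Runner zombie enemy that chases the first player pawn across the X-Z plane of a Paper2D scene.
; Each tick it normalizes the direction to the player and moves at a fixed speed, never along Y.
; X and Z are applied as separate swept offsets, so a block on one axis does not stop the other.
; The flipbook faces the chase direction by mirroring its X scale, negative when the player is toward +X.
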(event EventBeginPlay)

(event EventTick
  (params (DeltaSeconds :type Float%20%28single-precision%29))
  (bind _returnvalue (Game|Player|GetPlayerPawn 0))
  (bind _returnvalue_2 (Transformation|GetActorLocation))
  (bind _returnvalue_3 (Transformation|GetActorLocation _returnvalue))
  (bind _returnvalue_4 (- _returnvalue_3 _returnvalue_2))
  (bind _returnvalue_5 (Math|Vector|Normalize _returnvalue_4))
  (bind (_x _y _z) (Math|Vector|BreakVector _returnvalue_5))
  (Transformation|AddActorWorldOffset (Math|Vector|MakeVector (* (* _x 105.0) DeltaSeconds) 0.0 0.0) true)
  (Transformation|AddActorWorldOffset (Math|Vector|MakeVector 0.0 0.0 (* (* _z 105.0) DeltaSeconds)) true)
  (Transformation|SetRelativeScale3D (Actor|GetComponentbyClass "/Script/Paper2D.PaperFlipbookComponent") (Math|Vector|MakeVector (Math|Float|SelectFloat -0.45 0.45 (> _x 0.0)) 0.45 0.45)))

(fn ConstructionScript)