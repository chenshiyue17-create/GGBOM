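; Mutant hound enemy for a 2D Paper2D game on the X-Z plane that chases the player.
; Tick steers it with swept X and Z moves toward a point beside the player on its current side, picking a run flipbook by dominant direction.
; On arrival it only shows the down-facing pounce flipbook, with no attack logic.
; Non-player overlaps push it away, and damage reduces CurrentHealth until it is destroyed.
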(event EventBeginPlay)

(event Collision|EventActorBeginOverlap
  (params (OtherActor :type Actor%20Object%20Reference))
  (if (!= OtherActor (Game|Player|GetPlayerPawn 0))
    (Transformation|AddActorWorldOffset (* (Math|Vector|Normalize (- (Transformation|GetActorLocation) (Transformation|GetActorLocation OtherActor))) "40.0, 0.0, 40.0"))))

(event EventTick
  (params (DeltaSeconds :type Float%20%28single-precision%29))
  (bind _returnvalue (Game|Player|GetPlayerPawn 0))
  (bind _returnvalue_2 (Transformation|GetActorLocation))
  (bind _returnvalue_3 (Actor|GetComponentbyClass "/Script/Paper2D.PaperFlipbookComponent"))
  (bind _returnvalue_4 (Transformation|GetActorLocation _returnvalue))
  (bind _returnvalue_5 (- _returnvalue_2 _returnvalue_4))
  (bind _x (Math|Vector|BreakVector _returnvalue_5))
  (bind _returnvalue_6 (Math|Vector|MakeVector _x 0.0 0.0))
  (bind _returnvalue_7 (Math|Vector|Normalize _returnvalue_6))
  (bind _returnvalue_8 (* _returnvalue_7 "110.0, 0.0, -10.0"))
  (bind _returnvalue_9 (+ _returnvalue_4 _returnvalue_8))
  (bind _returnvalue_10 (- _returnvalue_9 _returnvalue_2))
  (bind _returnvalue_11 (Math|Vector|Normalize _returnvalue_10))
  (bind (_x_2 _y _z) (Math|Vector|BreakVector _returnvalue_11))
  (if (> (Math|Vector|Distance(Vector) _returnvalue_9 _returnvalue_2) 8e+01)
    (Transformation|AddActorWorldOffset (Math|Vector|MakeVector (* (* _x_2 1.5e+02) DeltaSeconds) 0.0 0.0) true)
    (Transformation|AddActorWorldOffset (Math|Vector|MakeVector 0.0 0.0 (* (* _z 1.5e+02) DeltaSeconds)) true)
    (if (> (Math|Float|Absolute(Float) _x_2) (Math|Float|Absolute(Float) _z))
      (if (> _x_2 0.0)
        (Sprite|SetFlipbook _returnvalue_3 "/Game/P01/Imported/Content/Asset/Art/02_Enemies/MutantHound/Run/Dir_02_Right/Flipbooks/FB_T_Hound_Run_Dir_02_Right_Sheet.FB_T_Hound_Run_Dir_02_Right_Sheet")
        (else
          (Sprite|SetFlipbook _returnvalue_3 "/Game/P01/Imported/Content/Asset/Art/02_Enemies/MutantHound/Run/Dir_04_Left/Flipbooks/FB_T_Hound_Run_Dir_04_Left_Sheet.FB_T_Hound_Run_Dir_04_Left_Sheet")))
      (elif (> _z 0.0)
        (Sprite|SetFlipbook _returnvalue_3 "/Game/P01/Imported/Content/Asset/Art/02_Enemies/MutantHound/Run/Dir_03_Up/Flipbooks/FB_T_Hound_Run_Dir_03_Up_Sheet.FB_T_Hound_Run_Dir_03_Up_Sheet")
        (else
          (Sprite|SetFlipbook _returnvalue_3 "/Game/P01/Imported/Content/Asset/Art/02_Enemies/MutantHound/Run/Dir_01_Down/Flipbooks/FB_T_Hound_Run_Dir_01_Down_Sheet.FB_T_Hound_Run_Dir_01_Down_Sheet"))))
    (else
      (Sprite|SetFlipbook _returnvalue_3 "/Game/P01/Imported/Content/Asset/Art/02_Enemies/MutantHound/Pounce/Dir_01_Down/Flipbooks/FB_T_Hound_Pounce_Dir_01_Down_Sheet.FB_T_Hound_Pounce_Dir_01_Down_Sheet"))))

(event Game|Damage|EventAnyDamage
  (params (Damage :type Float%20%28single-precision%29) (DamageType :type Damage%20Type%20Object%20Reference) (InstigatedBy :type Controller%20Object%20Reference) (DamageCauser :type Actor%20Object%20Reference))
  (Variables|战斗属性|SetCurrentHealth (- (Variables|战斗属性|GetCurrentHealth) Damage))
  (if (<= (- (Variables|战斗属性|GetCurrentHealth) Damage) 0.0)
    (Actor|DestroyActor)))

(fn ConstructionScript)